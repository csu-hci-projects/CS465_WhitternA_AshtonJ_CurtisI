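; FittSphere is a VR target sphere for a Fitts' law reaction test.
; StartRound and NextTarget pick random spheres, and HighlightAsTarget turns the pick red and the others black.
; A target overlap logs distance to the VRPawn's right-hand trigger and a time (StartTime is set at overlap), turns green, then advances after a delay.
; While the hit count is below 13, each hit writes the samples to JSON via VaRest.
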(event Custom|StartRound
  ;[1 1 1] Start Logic
  (Development|PrintString "Round 1 Starting...")
  (bind _outactors (Actor|GetAllActorsOfClass "FittSphere_C"))
  (bind _output_get (Variables|Default|SetCurrentTarget (Utilities|Array|Get(acopy) _outactors (Math|Random|RandomIntegerinRange 0 (Utilities|Array|Length _outactors)))))
  (CallFunction|HighlightasTarget _output_get))

(event Custom|NextTarget
  ;[1 1 1] Next Target Logic
  (bind _outactors (Actor|GetAllActorsOfClass "FittSphere_C"))
  (for _array_element _outactors
    (if (not (Variables|Default|GetHit))
      (Utilities|Array|Add (Variables|Default|GetValidSpheres) _array_element)))
  (CallFunction|HighlightasTarget (Utilities|Array|Get(acopy) (Variables|Default|GetValidSpheres) (Math|Random|RandomIntegerinRange 0 (Utilities|Array|Length (Variables|Default|GetValidSpheres))))))

(event Collision|EventActorBeginOverlap
  (params (OtherActor :type Actor%20Object%20Reference))
  (Development|PrintString "HHHHIIIIITTTTT")
  (if (Utilities|IsValid (Variables|Default|GetCurrentTarget))
    (if (Variables|Default|GetIsTarget)
      (Math|Integer|IncrementInt (Variables|Default|GetObjCount)
        (:%20%20
          (Variables|Default|SetStartTime (Utilities|Time|GetTimeSeconds))
          (bind _output_get (Variables|Default|SetReactionTime (- (Utilities|Time|GetTimeSeconds) (Variables|Default|GetStartTime))))
          (bind _asvrpawn (Utilities|Casting|CastToVRPawn OtherActor))
          (bind _output_get_2 (Variables|Default|SetDistance (Math|Vector|VectorLength (- (Transformation|GetWorldLocation (Variables|Default|GetSphere)) (Transformation|GetWorldLocation (Variables|/Game/VRTemplate/Blueprints/VRPawn.VRPawn_C|GetRightHandTrigger _asvrpawn))))))
          (Utilities|Array|Add (Variables|Default|GetArrayofData) (Utilities|Struct|MakeFittsData _output_get_2 _output_get))
          (Rendering|Material|SetMaterial (Variables|FittSphere_C|GetSphere (Variables|Default|GetCurrentTarget)) 0 "/Engine/EngineDebugMaterials/VertexColorViewMode_GreenOnly.VertexColorViewMode_GreenOnly")
          (Utilities|FlowControl|Delay 2.0)
          (Rendering|Material|SetMaterial (Variables|Default|GetSphere) 0 0)
          (Variables|Default|SetIsTarget false)
          (Variables|Default|SetHit true)
          (CallFunction|NextTarget)
          (if (> 13 (Variables|Default|GetObjCount))
            (Development|PrintString "Round Complete.")
            ;[1 1 1] Writing Data to File
            (bind _returnvalue (Class|VaRestSubsystem|ConstructVaRestJsonObject (|VaRestSubsystem)))
            (bind _output_get_3 (Variables|Default|SetLevel1Data _returnvalue))
            (for _array_element (Variables|Default|GetArrayofData)
              (bind _returnvalue_2 (Class|VaRestSubsystem|ConstructVaRestJsonObject (|VaRestSubsystem)))
              (bind _output_get_4 (Variables|Default|SetTempJSON _returnvalue_2))
              (Class|VaRestJsonObject|SetNumberField (Variables|Default|GetTempJSON) "Distance" (.Distance (Utilities|Struct|BreakFittsData _array_element)))
              (Class|VaRestJsonObject|SetNumberField (Variables|Default|GetTempJSON) "Reaction Time" (.Time (Utilities|Struct|BreakFittsData _array_element)))
              (Utilities|Array|Add (Variables|Default|GetVAarray) (Class|VaRestSubsystem|ConstructJsonValueObject (|VaRestSubsystem) _output_get_4)))
            (Class|VaRestJsonObject|SetArrayField _output_get_3 "Level1Data" (Variables|Default|GetVAarray))
            (Class|VaRestJsonObject|WritetoFilePath _returnvalue "Level1Output" true)
            (Development|PrintString "Wrote to File.")))))
    (else
      (Development|PrintString "NNNNNOOOOOPPPPPEEEE"))))

(fn ConstructionScript)

(fn HighlightasTarget
  (bind _outactors (Actor|GetAllActorsOfClass "FittSphere_C"))
  (for _array_element _outactors
    (Variables|Default|SetIsTarget false)
    (Rendering|Material|SetMaterial (Variables|FittSphere_C|GetSphere _array_element) 0 "/Engine/EngineDebugMaterials/BlackUnlitMaterial.BlackUnlitMaterial")
    (Rendering|Material|SetMaterial (Variables|Default|GetSphere) 0 "/Engine/EngineDebugMaterials/VertexColorViewMode_RedOnly.VertexColorViewMode_RedOnly")
    (Variables|Default|SetCurrentTarget (Variables|Default|GetCurrentTarget))
    (Variables|Default|SetIsTarget true)))