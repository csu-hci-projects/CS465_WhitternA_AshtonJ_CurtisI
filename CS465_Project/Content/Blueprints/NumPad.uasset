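; VR number pad for a typing trial in which the player enters randomly generated digit sequences by touch.
; Box overlaps from VRPawn append digits, debounced by a shared IsPressed flag, and log hit location, time since previous press and digit in parallel arrays.
; Delete drops the last entry; Enter checks the target, discarding a wrong attempt's data or counting a pass, and writes the arrays to JSON after three passes.
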(event OnComponentBeginOverlap(Box11)
  (params (OverlappedComponent :type Primitive%20Component%20Object%20Reference) (OtherActor :type Actor%20Object%20Reference) (OtherComp :type Primitive%20Component%20Object%20Reference) (OtherBodyIndex :type Integer) (bFromSweep :type Boolean) (SweepResult :type Hit%20Result%20Structure%20%28by%20ref%29))
  (bind _time_array (Variables|Default|GetTime%20Array))
  (bind _numbertext (Variables|Default|GetNumberText))
  (bind _coordinates (Variables|Default|GetCoordinates))
  (bind _numbershit (Variables|Default|GetNumbersHit))
  ;[0.151 0.151 0.151] Delete
  (Utilities|Casting|CastToVRPawn OtherActor)
  (Rendering|Components|TextRender|SetText _numbertext (Utilities|Text|ToText(String) (Utilities|String|LeftChop (Utilities|String|ToString(Text) (Variables|/Script/Engine.TextRenderComponent|GetText _numbertext)) 1)))
  (Utilities|Array|RemoveIndex _coordinates (Utilities|Array|LastIndex _coordinates))
  (Utilities|Array|RemoveIndex _time_array (Utilities|Array|LastIndex _time_array))
  (Utilities|Array|RemoveIndex _numbershit (Utilities|Array|LastIndex _numbershit))
  (Variables|Default|SetDeltaTime (- (Actor|GetGameTimeSinceCreation) (Variables|Default|GetPrevious%20Press%20Time))))

(event OnComponentBeginOverlap(Box12)
  (params (OverlappedComponent :type Primitive%20Component%20Object%20Reference) (OtherActor :type Actor%20Object%20Reference) (OtherComp :type Primitive%20Component%20Object%20Reference) (OtherBodyIndex :type Integer) (bFromSweep :type Boolean) (SweepResult :type Hit%20Result%20Structure%20%28by%20ref%29))
  (bind _coordinates (Variables|Default|GetCoordinates))
  (bind _targetnumber (Variables|Default|GetTargetNumber))
  (bind _numbertext (Variables|Default|GetNumberText))
  (bind _time_array (Variables|Default|GetTime%20Array))
  (bind _coordinates_2 (Variables|Default|GetCoordinates))
  (bind _numbershit (Variables|Default|GetNumbersHit))
  (bind _returnvalue (Utilities|Array|Length _coordinates_2))
  (bind _text (Variables|/Script/Engine.TextRenderComponent|GetText _numbertext))
  (bind _returnvalue_2 (Utilities|String|ToString(Text) _text))
  ;[0.1406 0.1406 0.1406] Enter
  (if (== (Math|Conversions|ToInteger(Byte) (Utilities|String|ToString(Text) (Variables|/Script/Engine.TextRenderComponent|GetText (Variables|Default|GetTargetNumber)))) (Math|Conversions|ToInteger(Byte) _returnvalue_2))
    ;[0.1667 0.1667 0.1667] If User has completed 3 runs corectly,. end simulation and write data to a file, otherwise generate next set of numbers
    (bind _result (Math|Integer|IncrementInt (Variables|Default|GetPassed%20Count))
      (:%20%20
        (if (< _result 3)
          (Rendering|Components|TextRender|SetText (Variables|Default|GetNumberText) (Utilities|Text|ToText(String) (Utilities|String|MakeLiteralString)))
          (Rendering|Components|TextRender|SetText (Variables|Default|GetTargetNumber) (Utilities|Text|ToText(String) (Utilities|String|MakeLiteralString)))
          (for _index (range 0 9)
            (Rendering|Components|TextRender|SetText _targetnumber (Utilities|Text|ToText(String) (Utilities|String|Append (Utilities|String|ToString(Text) (Variables|/Script/Engine.TextRenderComponent|GetText _targetnumber)) (Utilities|String|ToString(Text) (Utilities|Text|ToText(Integer) (Math|Random|RandomIntegerinRange 0 9)))))))
          (else
            (Rendering|Components|TextRender|SetText (Variables|Default|GetTargetNumber) (Utilities|Text|ToText(String) (Utilities|String|MakeLiteralString "All Trials Passed")))
            (Class|VaRestJsonObject|WritetoFilePath (|MakeJson (Variables|Default|GetCoordinates) (Variables|Default|GetTime%20Array) (Variables|Default|GetNumbersHit)) "Level1_outputData.json" true)))))
    (else
      ;[0.1562 0.1562 0.1562] If nUmber Sequence is Incorrect, tell user and remove recorded data
      (for _index_2 (range (- _returnvalue (Utilities|String|Len _returnvalue_2)) _returnvalue)
        (Utilities|Array|RemoveIndex _time_array (Utilities|Array|LastIndex _time_array))
        (Utilities|Array|RemoveIndex _coordinates (Utilities|Array|LastIndex _coordinates))
        (Utilities|Array|RemoveIndex _numbershit (Utilities|Array|LastIndex _numbershit)))
      (Rendering|Components|TextRender|SetText _numbertext (Utilities|Text|ToText(String) (Utilities|String|MakeLiteralString "Incorrect")))
      (Utilities|FlowControl|Delay 1.0)
      (Rendering|Components|TextRender|SetText _numbertext (Utilities|Text|ToText(String) (Utilities|String|MakeLiteralString))))))

(event OnComponentEndOverlap(Box1)
  (params (OverlappedComponent :type Primitive%20Component%20Object%20Reference) (OtherActor :type Actor%20Object%20Reference) (OtherComp :type Primitive%20Component%20Object%20Reference) (OtherBodyIndex :type Integer))
  (Variables|Default|SetIsPressed false))

(event OnComponentEndOverlap(Box4)
  (params (OverlappedComponent :type Primitive%20Component%20Object%20Reference) (OtherActor :type Actor%20Object%20Reference) (OtherComp :type Primitive%20Component%20Object%20Reference) (OtherBodyIndex :type Integer))
  (Variables|Default|SetIsPressed false))

(event OnComponentEndOverlap(Box3)
  (params (OverlappedComponent :type Primitive%20Component%20Object%20Reference) (OtherActor :type Actor%20Object%20Reference) (OtherComp :type Primitive%20Component%20Object%20Reference) (OtherBodyIndex :type Integer))
  (Variables|Default|SetIsPressed false))

(event OnComponentEndOverlap(Box2)
  (params (OverlappedComponent :type Primitive%20Component%20Object%20Reference) (OtherActor :type Actor%20Object%20Reference) (OtherComp :type Primitive%20Component%20Object%20Reference) (OtherBodyIndex :type Integer))
  (Variables|Default|SetIsPressed false))

(event OnComponentEndOverlap(Box5)
  (params (OverlappedComponent :type Primitive%20Component%20Object%20Reference) (OtherActor :type Actor%20Object%20Reference) (OtherComp :type Primitive%20Component%20Object%20Reference) (OtherBodyIndex :type Integer))
  (Variables|Default|SetIsPressed false))

(event OnComponentEndOverlap(Box8)
  (params (OverlappedComponent :type Primitive%20Component%20Object%20Reference) (OtherActor :type Actor%20Object%20Reference) (OtherComp :type Primitive%20Component%20Object%20Reference) (OtherBodyIndex :type Integer))
  (Variables|Default|SetIsPressed false))

(event OnComponentEndOverlap(Box7)
  (params (OverlappedComponent :type Primitive%20Component%20Object%20Reference) (OtherActor :type Actor%20Object%20Reference) (OtherComp :type Primitive%20Component%20Object%20Reference) (OtherBodyIndex :type Integer))
  (Variables|Default|SetIsPressed false))

(event OnComponentEndOverlap(Box10)
  (params (OverlappedComponent :type Primitive%20Component%20Object%20Reference) (OtherActor :type Actor%20Object%20Reference) (OtherComp :type Primitive%20Component%20Object%20Reference) (OtherBodyIndex :type Integer))
  (Variables|Default|SetIsPressed false))

(event OnComponentEndOverlap(Box9)
  (params (OverlappedComponent :type Primitive%20Component%20Object%20Reference) (OtherActor :type Actor%20Object%20Reference) (OtherComp :type Primitive%20Component%20Object%20Reference) (OtherBodyIndex :type Integer))
  (Variables|Default|SetIsPressed false))

(event OnComponentBeginOverlap(Box5)
  (params (OverlappedComponent :type Primitive%20Component%20Object%20Reference) (OtherActor :type Actor%20Object%20Reference) (OtherComp :type Primitive%20Component%20Object%20Reference) (OtherBodyIndex :type Integer) (bFromSweep :type Boolean) (SweepResult :type Hit%20Result%20Structure%20%28by%20ref%29))
  (bind _numbertext (Variables|Default|GetNumberText))
  ;[0.2344 0.2344 0.2344] Number button functionality
  (Utilities|Casting|CastToVRPawn OtherActor)
  (if (not (Variables|Default|GetIsPressed))
    (Variables|Default|SetIsPressed true)
    (CallFunction|ButtonHit (Transformation|GetWorldLocation OtherComp))
    (Rendering|Components|TextRender|SetText _numbertext (Utilities|Text|ToText(String) (Utilities|String|Append (Utilities|String|ToString(Text) (Variables|/Script/Engine.TextRenderComponent|GetText _numbertext)) (Utilities|String|ToString(Text) (Variables|/Script/Engine.TextRenderComponent|GetText (Variables|Default|GetText5))))))
    (Utilities|Array|Add (Variables|Default|GetNumbersHit) 5.0)))

(event OnComponentBeginOverlap(Box6)
  (params (OverlappedComponent :type Primitive%20Component%20Object%20Reference) (OtherActor :type Actor%20Object%20Reference) (OtherComp :type Primitive%20Component%20Object%20Reference) (OtherBodyIndex :type Integer) (bFromSweep :type Boolean) (SweepResult :type Hit%20Result%20Structure%20%28by%20ref%29))
  (bind _numbertext (Variables|Default|GetNumberText))
  ;[0.2344 0.2344 0.2344] Number button functionality
  (Utilities|Casting|CastToVRPawn OtherActor)
  (if (not (Variables|Default|GetIsPressed))
    (Variables|Default|SetIsPressed true)
    (CallFunction|ButtonHit (Transformation|GetWorldLocation OtherComp))
    (Rendering|Components|TextRender|SetText _numbertext (Utilities|Text|ToText(String) (Utilities|String|Append (Utilities|String|ToString(Text) (Variables|/Script/Engine.TextRenderComponent|GetText _numbertext)) (Utilities|String|ToString(Text) (Variables|/Script/Engine.TextRenderComponent|GetText (Variables|Default|GetText6))))))
    (Utilities|Array|Add (Variables|Default|GetNumbersHit) 6.0)))

(event OnComponentBeginOverlap(Box1)
  (params (OverlappedComponent :type Primitive%20Component%20Object%20Reference) (OtherActor :type Actor%20Object%20Reference) (OtherComp :type Primitive%20Component%20Object%20Reference) (OtherBodyIndex :type Integer) (bFromSweep :type Boolean) (SweepResult :type Hit%20Result%20Structure%20%28by%20ref%29))
  (bind _numbertext (Variables|Default|GetNumberText))
  ;[0.2344 0.2344 0.2344] Number button functionality
  (Utilities|Casting|CastToVRPawn OtherActor)
  (if (not (Variables|Default|GetIsPressed))
    (Variables|Default|SetIsPressed true)
    (CallFunction|ButtonHit (Transformation|GetWorldLocation OtherComp))
    (Rendering|Components|TextRender|SetText _numbertext (Utilities|Text|ToText(String) (Utilities|String|Append (Utilities|String|ToString(Text) (Variables|/Script/Engine.TextRenderComponent|GetText _numbertext)) (Utilities|String|ToString(Text) (Variables|/Script/Engine.TextRenderComponent|GetText (Variables|Default|GetText1))))))
    (Utilities|Array|Add (Variables|Default|GetNumbersHit) 1.0)))

(event OnComponentBeginOverlap(Box4)
  (params (OverlappedComponent :type Primitive%20Component%20Object%20Reference) (OtherActor :type Actor%20Object%20Reference) (OtherComp :type Primitive%20Component%20Object%20Reference) (OtherBodyIndex :type Integer) (bFromSweep :type Boolean) (SweepResult :type Hit%20Result%20Structure%20%28by%20ref%29))
  (bind _numbertext (Variables|Default|GetNumberText))
  ;[0.2344 0.2344 0.2344] Number button functionality
  (Utilities|Casting|CastToVRPawn OtherActor)
  (if (not (Variables|Default|GetIsPressed))
    (Variables|Default|SetIsPressed true)
    (CallFunction|ButtonHit (Transformation|GetWorldLocation OtherComp))
    (Rendering|Components|TextRender|SetText _numbertext (Utilities|Text|ToText(String) (Utilities|String|Append (Utilities|String|ToString(Text) (Variables|/Script/Engine.TextRenderComponent|GetText _numbertext)) (Utilities|String|ToString(Text) (Variables|/Script/Engine.TextRenderComponent|GetText (Variables|Default|GetText4))))))
    (Utilities|Array|Add (Variables|Default|GetNumbersHit) 4.0)))

(event OnComponentBeginOverlap(Box3)
  (params (OverlappedComponent :type Primitive%20Component%20Object%20Reference) (OtherActor :type Actor%20Object%20Reference) (OtherComp :type Primitive%20Component%20Object%20Reference) (OtherBodyIndex :type Integer) (bFromSweep :type Boolean) (SweepResult :type Hit%20Result%20Structure%20%28by%20ref%29))
  (bind _numbertext (Variables|Default|GetNumberText))
  ;[0.2344 0.2344 0.2344] Number button functionality
  (Utilities|Casting|CastToVRPawn OtherActor)
  (if (not (Variables|Default|GetIsPressed))
    (Variables|Default|SetIsPressed true)
    (CallFunction|ButtonHit (Transformation|GetWorldLocation OtherComp))
    (Rendering|Components|TextRender|SetText _numbertext (Utilities|Text|ToText(String) (Utilities|String|Append (Utilities|String|ToString(Text) (Variables|/Script/Engine.TextRenderComponent|GetText _numbertext)) (Utilities|String|ToString(Text) (Variables|/Script/Engine.TextRenderComponent|GetText (Variables|Default|GetText3))))))
    (Utilities|Array|Add (Variables|Default|GetNumbersHit) 3.0)))

(event OnComponentBeginOverlap(Box2)
  (params (OverlappedComponent :type Primitive%20Component%20Object%20Reference) (OtherActor :type Actor%20Object%20Reference) (OtherComp :type Primitive%20Component%20Object%20Reference) (OtherBodyIndex :type Integer) (bFromSweep :type Boolean) (SweepResult :type Hit%20Result%20Structure%20%28by%20ref%29))
  (bind _numbertext (Variables|Default|GetNumberText))
  ;[0.2344 0.2344 0.2344] Number button functionality
  (Utilities|Casting|CastToVRPawn OtherActor)
  (if (not (Variables|Default|GetIsPressed))
    (Variables|Default|SetIsPressed true)
    (CallFunction|ButtonHit (Transformation|GetWorldLocation OtherComp))
    (Rendering|Components|TextRender|SetText _numbertext (Utilities|Text|ToText(String) (Utilities|String|Append (Utilities|String|ToString(Text) (Variables|/Script/Engine.TextRenderComponent|GetText _numbertext)) (Utilities|String|ToString(Text) (Variables|/Script/Engine.TextRenderComponent|GetText (Variables|Default|GetText2))))))
    (Utilities|Array|Add (Variables|Default|GetNumbersHit) 2.0)))

(event OnComponentEndOverlap(Box6)
  (params (OverlappedComponent :type Primitive%20Component%20Object%20Reference) (OtherActor :type Actor%20Object%20Reference) (OtherComp :type Primitive%20Component%20Object%20Reference) (OtherBodyIndex :type Integer))
  (Variables|Default|SetIsPressed false))

(event OnComponentBeginOverlap(Box8)
  (params (OverlappedComponent :type Primitive%20Component%20Object%20Reference) (OtherActor :type Actor%20Object%20Reference) (OtherComp :type Primitive%20Component%20Object%20Reference) (OtherBodyIndex :type Integer) (bFromSweep :type Boolean) (SweepResult :type Hit%20Result%20Structure%20%28by%20ref%29))
  (bind _numbertext (Variables|Default|GetNumberText))
  ;[0.2344 0.2344 0.2344] Number button functionality
  (Utilities|Casting|CastToVRPawn OtherActor)
  (if (not (Variables|Default|GetIsPressed))
    (Variables|Default|SetIsPressed true)
    (CallFunction|ButtonHit (Transformation|GetWorldLocation OtherComp))
    (Rendering|Components|TextRender|SetText _numbertext (Utilities|Text|ToText(String) (Utilities|String|Append (Utilities|String|ToString(Text) (Variables|/Script/Engine.TextRenderComponent|GetText _numbertext)) (Utilities|String|ToString(Text) (Variables|/Script/Engine.TextRenderComponent|GetText (Variables|Default|GetText8))))))
    (Utilities|Array|Add (Variables|Default|GetNumbersHit) 8.0)))

(event OnComponentBeginOverlap(Box7)
  (params (OverlappedComponent :type Primitive%20Component%20Object%20Reference) (OtherActor :type Actor%20Object%20Reference) (OtherComp :type Primitive%20Component%20Object%20Reference) (OtherBodyIndex :type Integer) (bFromSweep :type Boolean) (SweepResult :type Hit%20Result%20Structure%20%28by%20ref%29))
  (bind _numbertext (Variables|Default|GetNumberText))
  ;[0.2344 0.2344 0.2344] Number button functionality
  (Utilities|Casting|CastToVRPawn OtherActor)
  (if (not (Variables|Default|GetIsPressed))
    (Variables|Default|SetIsPressed true)
    (CallFunction|ButtonHit (Transformation|GetWorldLocation OtherComp))
    (Rendering|Components|TextRender|SetText _numbertext (Utilities|Text|ToText(String) (Utilities|String|Append (Utilities|String|ToString(Text) (Variables|/Script/Engine.TextRenderComponent|GetText _numbertext)) (Utilities|String|ToString(Text) (Variables|/Script/Engine.TextRenderComponent|GetText (Variables|Default|GetText7))))))
    (Utilities|Array|Add (Variables|Default|GetNumbersHit) 7.0)))

(event OnComponentBeginOverlap(Box10)
  (params (OverlappedComponent :type Primitive%20Component%20Object%20Reference) (OtherActor :type Actor%20Object%20Reference) (OtherComp :type Primitive%20Component%20Object%20Reference) (OtherBodyIndex :type Integer) (bFromSweep :type Boolean) (SweepResult :type Hit%20Result%20Structure%20%28by%20ref%29))
  (bind _numbertext (Variables|Default|GetNumberText))
  ;[0.2344 0.2344 0.2344] Number button functionality
  (Utilities|Casting|CastToVRPawn OtherActor)
  (if (not (Variables|Default|GetIsPressed))
    (Variables|Default|SetIsPressed true)
    (CallFunction|ButtonHit (Transformation|GetWorldLocation OtherComp))
    (Rendering|Components|TextRender|SetText _numbertext (Utilities|Text|ToText(String) (Utilities|String|Append (Utilities|String|ToString(Text) (Variables|/Script/Engine.TextRenderComponent|GetText _numbertext)) (Utilities|String|ToString(Text) (Variables|/Script/Engine.TextRenderComponent|GetText (Variables|Default|GetText10))))))
    (Utilities|Array|Add (Variables|Default|GetNumbersHit) 0.0)))

(event OnComponentBeginOverlap(Box9)
  (params (OverlappedComponent :type Primitive%20Component%20Object%20Reference) (OtherActor :type Actor%20Object%20Reference) (OtherComp :type Primitive%20Component%20Object%20Reference) (OtherBodyIndex :type Integer) (bFromSweep :type Boolean) (SweepResult :type Hit%20Result%20Structure%20%28by%20ref%29))
  (bind _numbertext (Variables|Default|GetNumberText))
  ;[0.2344 0.2344 0.2344] Number button functionality
  (Utilities|Casting|CastToVRPawn OtherActor)
  (if (not (Variables|Default|GetIsPressed))
    (Variables|Default|SetIsPressed true)
    (CallFunction|ButtonHit (Transformation|GetWorldLocation OtherComp))
    (Rendering|Components|TextRender|SetText _numbertext (Utilities|Text|ToText(String) (Utilities|String|Append (Utilities|String|ToString(Text) (Variables|/Script/Engine.TextRenderComponent|GetText _numbertext)) (Utilities|String|ToString(Text) (Variables|/Script/Engine.TextRenderComponent|GetText (Variables|Default|GetText9))))))
    (Utilities|Array|Add (Variables|Default|GetNumbersHit) 9.0)))

(event EventBeginPlay
  (bind _targetnumber (Variables|Default|GetTargetNumber))
  ;[0.276 0.276 0.276] Initialize Number to be typed in
  (Variables|Default|SetPrevious%20Press%20Time (Actor|GetGameTimeSinceCreation))
  (for _index (range 0 9)
    (Rendering|Components|TextRender|SetText _targetnumber (Utilities|Text|ToText(String) (Utilities|String|Append (Utilities|String|ToString(Text) (Variables|/Script/Engine.TextRenderComponent|GetText _targetnumber)) (Utilities|String|ToString(Text) (Utilities|Text|ToText(Integer) (Math|Random|RandomIntegerinRange 0 9))))))))

(fn ConstructionScript)

(fn RecordDistances
  (params (Start%20Vector :type Vector))
  (Utilities|Array|Add (Variables|Default|GetCoordinates) (Utilities|String|ToString(Vector) Start%20Vector))
  (Utilities|Array|Add (Variables|Default|GetTime%20Array) (Variables|Default|GetDeltaTime)))

(fn ButtonHit
  (params (Hit%20Location :type Vector))
  (bind _returnvalue (Actor|GetGameTimeSinceCreation))
  (Variables|Default|SetDeltaTime (- _returnvalue (Variables|Default|GetPrevious%20Press%20Time)))
  (Variables|Default|SetPrevious%20Press%20Time _returnvalue)
  (bind _output_get (Variables|Default|SetCurrent%20Hit Hit%20Location))
  (CallFunction|RecordDistances _output_get))